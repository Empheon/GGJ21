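; PirateGameInstance is a GameInstance Blueprint that manages the lifetime of the in-game HUD widget.
; ShowIngameHUD creates an IngameScreen widget for player controller 0, adds it to the viewport and stores it, only if none is already valid.
; CloseIngameHUD removes the stored widget from its parent and clears the reference.
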(event Custom|Show%20IngameHUD
  ;[1 1 1] Ingame Hud
  (Utilities|IsValid (Variables|Default|GetIngameHUD)
    (:Is%20Not%20Valid
      (bind _returnvalue (UserInterface|CreateWidget "/Game/Blueprints/UI/IngameScreen.IngameScreen_C" (Game|GetPlayerController 0)))
      (UserInterface|Viewport|AddtoViewport _returnvalue 0)
      (Variables|Default|SetIngameHUD _returnvalue))))

(event Custom|CloseIngameHUD
  ;[1 1 1] Ingame Hud
  (Utilities|IsValid (Variables|Default|GetIngameHUD)
    (:Is%20Valid
      (Widget|RemovefromParent (Variables|Default|GetIngameHUD))
      (Variables|Default|SetIngameHUD 0))))