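; Physics chest that pirate characters can stack and throw.
; On server-side overlap it notifies the pirate's stacking handler; stacking disables its physics and collision.
; Throwing launches it along its forward vector, ignoring the Direction input, and blocks pawns until a Tick-driven timer restores overlap and clears the thrower.
; Hitting a pirate other than the thrower passes a horizontal hit direction to that pirate and destroys the chest.
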(event OnComponentHit(Chest)
  (params (HitComponent :type Primitive%20Component%20Object%20Reference) (OtherActor :type Actor%20Object%20Reference) (OtherComp :type Primitive%20Component%20Object%20Reference) (NormalImpulse :type Vector :default "0, 0, 0") (Hit :type Hit%20Result%20Structure%20%28by%20ref%29))
  (bind _returnvalue (Transformation|GetActorLocation))
  (bind _returnvalue_2 (Transformation|GetActorLocation OtherActor))
  (bind _returnvalue_3 (- _returnvalue_2 _returnvalue))
  (bind _returnvalue_4 (Math|Vector|Normalize _returnvalue_3))
  (bind (_x _y) (Math|Vector|BreakVector _returnvalue_4))
  (if (!= OtherActor (Variables|Default|GetThrower))
    (bind _aspirate_character (Utilities|Casting|CastToPirateCharacter OtherActor))
    (Default|OnHitChest _aspirate_character (Math|Vector|MakeVector _x _y 0.0))
    (Actor|DestroyActor)))

(event Custom|OnThrow
  (params (Direction :type Vector) (Thrower :type Pirate%20Character%20Object%20Reference))
  (bind _chest (Variables|Default|GetChest))
  (Variables|Default|SetThrower Thrower)
  (Collision|SetCollisionResponsetoChannel _chest "ECC_Pawn" "ECR_Block")
  (Collision|SetCollisionEnabled _chest "QueryAndPhysics")
  (Physics|SetSimulatePhysics _chest true)
  (Physics|AddImpulse _chest (* (Transformation|GetActorForwardVector) 2e+03) "None" true)
  (Variables|Default|SetThrowTimer 2.0))

(event Custom|OnChestStacked
  (bind _chest (Variables|Default|GetChest))
  (Physics|SetSimulatePhysics _chest false)
  (Collision|SetCollisionEnabled _chest "NoCollision"))

(event Collision|EventActorBeginOverlap
  (params (OtherActor :type Actor%20Object%20Reference))
  (Networking|SwitchHasAuthority
    (:Authority
      (bind _aspirate_character (Utilities|Casting|CastToPirateCharacter OtherActor))
      (Default|OnChestStacked _aspirate_character self))))

(event EventTick
  (params (DeltaSeconds :type Float%20%28single-precision%29))
  (if (> (Variables|Default|GetThrowTimer) 0.0)
    (bind _output_get (Variables|Default|SetThrowTimer (Math|Float|Max(Float) (- (Variables|Default|GetThrowTimer) DeltaSeconds) 0.0)))
    (if (<= _output_get 0.0)
      (Collision|SetCollisionResponsetoChannel (Variables|Default|GetChest) "ECC_Pawn" "ECR_Overlap")
      (Variables|Default|SetThrower 0))))

(fn ConstructionScript)