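; Hole is an interactable dig spot that pirates dig to uncover a Chest, active only during one specific game state.
; Overlap sets or clears the pirate's CurrentInteractible and toggles InteractionText for player pawn 0, with Tick billboarding the text toward the camera.
; OnUse plays the dig montage while blocking movement through a counter, restored on completion or interruption.
; On completion, only the authority spawns the Chest and destroys the hole.
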(event EventBeginPlay
  (Rendering|SetVisibility (Variables|Default|GetInteraction%20text) false false))

(event Collision|EventActorBeginOverlap
  (params (OtherActor :type Actor%20Object%20Reference))
  (bind _asgame_state_pirate (Utilities|Casting|CastToGameStatePirate (Game|GetGameState)))
  (if (Utilities|Enum|Equal(Enum) (Variables|/Game/Blueprints/System/GameStatePirate.GameStatePirate_C|GetGameState _asgame_state_pirate) "NewEnumerator1")
    (bind _aspirate_character (Utilities|Casting|CastToPirateCharacter OtherActor))
    (Variables|/Game/Blueprints/System/PirateCharacter.PirateCharacter_C|SetCurrentInteractible _aspirate_character self)
    (bind _aspirate_character_2 (Utilities|Casting|CastToPirateCharacter (Game|Player|GetPlayerPawn 0)))
    (if (== _aspirate_character_2 _aspirate_character)
      (Rendering|SetVisibility (Variables|Default|GetInteraction%20text) true false))))

(event EventTick
  (params (DeltaSeconds :type Float%20%28single-precision%29))
  (Transformation|SetWorldRotation (Variables|Default|GetInteraction%20text) (Math|Conversions|RotationFromXVector (* (Transformation|GetActorForwardVector (Game|GetPlayerCameraManager 0)) -1.0)) false false))

(event Collision|EventActorEndOverlap
  (params (OtherActor :type Actor%20Object%20Reference))
  (bind _asgame_state_pirate (Utilities|Casting|CastToGameStatePirate (Game|GetGameState)))
  (if (Utilities|Enum|Equal(Enum) (Variables|/Game/Blueprints/System/GameStatePirate.GameStatePirate_C|GetGameState _asgame_state_pirate) "NewEnumerator1")
    (bind _aspirate_character (Utilities|Casting|CastToPirateCharacter OtherActor))
    (Variables|/Game/Blueprints/System/PirateCharacter.PirateCharacter_C|SetCurrentInteractible _aspirate_character 0)
    (bind _aspirate_character_2 (Utilities|Casting|CastToPirateCharacter (Game|Player|GetPlayerPawn 0)))
    (if (== _aspirate_character_2 _aspirate_character)
      (Rendering|SetVisibility (Variables|Default|GetInteraction%20text) false false))))

(event EventOnUse
  (params (Pawn :type Pirate%20Character%20Object%20Reference))
  (bind _disablemovementcount (Variables|/Game/Blueprints/System/PirateCharacter.PirateCharacter_C|GetDisableMovementCount Pawn))
  (bind _asgame_state_pirate (Utilities|Casting|CastToGameStatePirate (Game|GetGameState)))
  (if (Utilities|Enum|Equal(Enum) (Variables|/Game/Blueprints/System/GameStatePirate.GameStatePirate_C|GetGameState _asgame_state_pirate) "NewEnumerator1")
    (Math|Integer|IncrementInt _disablemovementcount
      (:%20%20
        (Animation|Montage|PlayMontage (Variables|/Script/Engine.Character|GetMesh Pawn) "/Game/Mesh/Character/Dig_Montage.Dig_Montage"
          (:OnCompleted
            (Math|Integer|DecrementInt _disablemovementcount
              (:%20%20
                (Networking|SwitchHasAuthority
                  (:Authority
                    (Game|SpawnActorfromClass "/Game/Blueprints/GameplayElement/Chest.Chest_C" (Math|Transform|MakeTransform (Transformation|GetActorLocation)) "AdjustIfPossibleButAlwaysSpawn" 0 0)
                    (Actor|DestroyActor))))))
          (:OnInterrupted
            (Math|Integer|DecrementInt _disablemovementcount)))))))

(fn ConstructionScript)