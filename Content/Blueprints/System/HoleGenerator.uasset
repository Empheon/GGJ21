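; HoleGenerator periodically spawns Hole actors inside configured map bounds, up to HoleLimit.
; A Tick countdown, once expired, prunes invalid HoleList entries and, below the limit, traces from a random XY at Z=0 toward a fixed point (0, 0, -1000).
; A hit spawns a hole at the impact point and resets the timer; otherwise checks repeat each tick, alongside a debug box draw.
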(event EventTick
  (params (DeltaSeconds :type Float%20%28single-precision%29))
  ;[1 1 1] Every x seconds
  (bind _output_get (Variables|Default|SetTimer (- (Variables|Default|GetTimer) DeltaSeconds)))
  (if (< _output_get 0.0)
    (Utilities|FlowControl|Sequence
      (:then_0
        ;[1 1 1] Remove if no longer exists
        (for (_array_element _array_index) (Variables|Default|GetHoleList)
          (Utilities|IsValid _array_element
            (:Is%20Not%20Valid
              (Utilities|Array|RemoveIndex (Variables|Default|GetHoleList) _array_index)))))
      (:then_1
        (if (< (Utilities|Array|Length (Variables|Default|GetHoleList)) (Variables|Default|GetHoleLimit))
          ;[1 1 1] Generate random transform
          (bind (_outhit _returnvalue) (Collision|LineTraceByChannel (Math|Vector|MakeVector (Math|Random|RandomFloatinRange (Variables|Default|GetMapMinLimitX) (Variables|Default|GetMapMaxLimitX)) (Math|Random|RandomFloatinRange (Variables|Default|GetMapMinLimitY) (Variables|Default|GetMapMaxLimitY)) 0.0) "0, 0,-1000.000000" "TraceTypeQuery1" false 0 "None"))
          (if _returnvalue
            (bind _returnvalue_2 (Game|SpawnActorfromClass "/Game/Blueprints/GameplayElement/Hole.Hole_C" (Math|Transform|MakeTransform (.ImpactPoint (Collision|BreakHitResult _outhit))) "AdjustIfPossibleButDontSpawnIfColliding" 0 0))
            (Utilities|Array|Add (Variables|Default|GetHoleList) _returnvalue_2)
            (Development|PrintString (Utilities|GetDisplayName _returnvalue_2))
            (Variables|Default|SetTimer (Variables|Default|GetDefaultTimer)))))
      (:then_2
        ;[1 1 1] Debug box
        (Rendering|Debug|DrawDebugBox :Extent (Math|Vector|MakeVector (- (Variables|Default|GetMapMaxLimitX) (Variables|Default|GetMapMinLimitX)) (- (Variables|Default|GetMapMaxLimitY) (Variables|Default|GetMapMinLimitY)) 0.0))))))

(event EventBeginPlay
  (Variables|Default|SetTimer (Variables|Default|GetDefaultTimer)))

(fn ConstructionScript)