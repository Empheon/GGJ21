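; PirateGameMode runs the match rules: it cycles a deposit zone on and off and ends the game when a player has enough chests.
; Tick counts down a timer held in GameStatePirate, alternately calling the zone spawn and destroy events and resetting the timer for each phase.
; Tick also checks every PlayerStatePirate's chest count against the winning condition, calling game over without a one-shot guard.
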(event EventBeginPlay
  (Utilities|FlowControl|Sequence
    (:then_0
      (bind _asgame_state_pirate (Utilities|Casting|CastToGameStatePirate (Game|GetGameState)))
      (Variables|Default|SetGame%20State%20Pirate _asgame_state_pirate))
    (:then_1
      (Variables|/Game/Blueprints/System/GameStatePirate.GameStatePirate_C|SetTimer (Variables|Default|GetGame%20State%20Pirate) (Variables|/Game/Blueprints/System/GameStatePirate.GameStatePirate_C|GetTimerUntilDepositZoneSpawn (Variables|Default|GetGame%20State%20Pirate))))))

(event EventTick
  (params (DeltaSeconds :type Float%20%28single-precision%29))
  (bind _game_state_pirate (Variables|Default|GetGame%20State%20Pirate))
  (bind _game_state_pirate_2 (Variables|Default|GetGame%20State%20Pirate))
  (bind _game_state_pirate_3 (Variables|Default|GetGame%20State%20Pirate))
  ;[1 1 1] Every x seconds
  (Utilities|FlowControl|Sequence
    (:then_0
      (bind _output_get (Variables|/Game/Blueprints/System/GameStatePirate.GameStatePirate_C|SetTimer _game_state_pirate (- (Variables|/Game/Blueprints/System/GameStatePirate.GameStatePirate_C|GetTimer _game_state_pirate) DeltaSeconds)))
      (if (Variables|/Game/Blueprints/System/GameStatePirate.GameStatePirate_C|GetDepositZoneIsActive _game_state_pirate)
        (if (< _output_get 0.0)
          (Default|CallDespositZoneDestroyEvent)
          (Variables|/Game/Blueprints/System/GameStatePirate.GameStatePirate_C|SetTimer (Variables|Default|GetGame%20State%20Pirate) (Variables|/Game/Blueprints/System/GameStatePirate.GameStatePirate_C|GetTimerUntilDepositZoneSpawn _game_state_pirate_3))
          (Variables|/Game/Blueprints/System/GameStatePirate.GameStatePirate_C|SetDepositZoneIsActive _game_state_pirate_2 false)
          (Development|PrintString "Depositve Zone is no longer active"))
        (elif (< _output_get 0.0)
          (Default|CallDespositZoneSpawnEvent)
          (Variables|/Game/Blueprints/System/GameStatePirate.GameStatePirate_C|SetTimer (Variables|Default|GetGame%20State%20Pirate) (Variables|/Game/Blueprints/System/GameStatePirate.GameStatePirate_C|GetDepositZoneLifeTime _game_state_pirate_3))
          (Variables|/Game/Blueprints/System/GameStatePirate.GameStatePirate_C|SetDepositZoneIsActive _game_state_pirate_2 true)
          (Development|PrintString "Deposite Zone is now active"))))
    (:then_1
      ;[1 1 1] Check if at least one player has more chests than the winning condition
      (for _array_element (Variables|/Script/Engine.GameStateBase|GetPlayerArray (Game|GetGameState))
        (bind _asplayer_state_pirate (Utilities|Casting|CastToPlayerStatePirate _array_element))
        (if (>= (Variables|/Game/Blueprints/System/PlayerStatePirate.PlayerStatePirate_C|GetNumberOfChests _asplayer_state_pirate) (Variables|/Game/Blueprints/System/GameStatePirate.GameStatePirate_C|GetWinningCondition (Variables|Default|GetGame%20State%20Pirate)))
          (Development|PrintString "The game is now finished")
          (Default|CallGameOverEvent))))))

(fn ConstructionScript)