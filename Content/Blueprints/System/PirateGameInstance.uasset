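; Game instance for a pirate game that manages top-level UI screens and starts or joins multiplayer games.
; Show/hide event pairs create and remove end-game, main menu and in-game HUD widgets through cached references, though only the in-game HUD clears its reference on close.
; Hosting stores the username, creates a session and opens Main as a listen server.
; Joining stores the username and connects by address through an "open" console command.
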(event Custom|ShowEndGame
  ;[1 1 1] Endgame
  (Utilities|IsValid (Variables|Default|GetEndGameHUD)
    (:Is%20Not%20Valid
      (bind _returnvalue (UserInterface|CreateWidget "/Game/Blueprints/UI/EndGameScreen.EndGameScreen_C" (Game|GetPlayerController 0)))
      (UserInterface|Viewport|AddtoViewport _returnvalue 0)
      (Variables|Default|SetEndGameHUD _returnvalue))))

(event Custom|HideEndGame
  (bind _endgamehud (Variables|Default|GetEndGameHUD))
  ;[1 1 1] Endgame
  (Utilities|IsValid _endgamehud
    (:Is%20Valid
      (Widget|RemovefromParent _endgamehud))))

(event Custom|Show%20IngameHUD
  ;[1 1 1] Ingame Hud
  (Utilities|IsValid (Variables|Default|GetIngameHUD)
    (:Is%20Not%20Valid
      (bind _returnvalue (UserInterface|CreateWidget "/Game/Blueprints/UI/IngameScreen.IngameScreen_C" (Game|GetPlayerController 0)))
      (UserInterface|Viewport|AddtoViewport _returnvalue 0)
      (Variables|Default|SetIngameHUD _returnvalue))))

(event Custom|CloseIngameHUD
  ;[1 1 1] Ingame Hud
  (Utilities|IsValid (Variables|Default|GetIngameHUD)
    (:Is%20Valid
      (Widget|RemovefromParent (Variables|Default|GetIngameHUD))
      (Variables|Default|SetIngameHUD 0))))

(event Custom|JoinGame
  (params (address :type String) (username :type String))
  (Variables|Default|SetUsername username)
  (Development|ExecuteConsoleCommand (Utilities|String|ToString(Text) (Utilities|Text|FormatText "open {ip}" (Utilities|Text|ToText(String) address))) (Game|GetPlayerController 0)))

(event Custom|ShowMainMenu
  ;[1 1 1] Ingame Hud
  (Utilities|IsValid (Variables|Default|GetMainMenuHUD)
    (:Is%20Not%20Valid
      (bind _returnvalue (UserInterface|CreateWidget "/Game/Blueprints/UI/MainMenu.MainMenu_C" (Game|GetPlayerController 0)))
      (UserInterface|Viewport|AddtoViewport _returnvalue 0)
      (Variables|Default|SetMainMenuHUD _returnvalue))))

(event Custom|HostGame
  (params (Username :type String))
  (Variables|Default|SetUsername Username)
  (|Session (Game|GetPlayerController 0) 0 false
    (:OnSuccess
      (Game|OpenLevel(byName) "Main" true "listen"))))

(event Custom|HideMainMenu
  (bind _mainmenuhud (Variables|Default|GetMainMenuHUD))
  ;[1 1 1] Ingame Hud
  (Utilities|IsValid _mainmenuhud
    (:Is%20Valid
      (Widget|RemovefromParent _mainmenuhud))))