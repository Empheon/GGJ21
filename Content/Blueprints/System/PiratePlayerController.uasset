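; Player controller for the pirate game that sets up the player's HUD and name and handles the ready toggle.
; On BeginPlay it shows the in-game HUD through the game instance, then passes the stored username to the game mode's ChangeName.
; The SetReady input calls a SetReady event, both gated on the first GameStatePirate state, which flips Ready on PlayerStatePirate.
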(event Custom|SetReady
  (bind _asgame_state_pirate (Utilities|Casting|CastToGameStatePirate (Game|GetGameState)))
  (if (Utilities|Enum|Equal(Enum) (Variables|/Game/Blueprints/System/GameStatePirate.GameStatePirate_C|GetGameState _asgame_state_pirate) "NewEnumerator0")
    (bind _asplayer_state_pirate (Utilities|Casting|CastToPlayerStatePirate (Variables|GetPlayerState)))
    (Variables|/Game/Blueprints/System/PlayerStatePirate.PlayerStatePirate_C|SetReady _asplayer_state_pirate (not (Variables|/Game/Blueprints/System/PlayerStatePirate.PlayerStatePirate_C|GetReady _asplayer_state_pirate)))))

(event Custom|SetPlayerName
  (params (Username :type String))
  (Class|GameModeBase|ChangeName (CallFunction|GetPirateGameMode) self Username false))

(event EventBeginPlay
  (Default|ShowIngameHUD (CallFunction|GetPirateGameInstance))
  (CallFunction|SetPlayerName (Variables|/Game/Blueprints/System/PirateGameInstance.PirateGameInstance_C|GetUsername (CallFunction|GetPirateGameInstance))))

(event Input|ActionEvents|InputActionSetReady
  (params (Key :type Key%20Structure :default "None"))
  (:Pressed
    (bind _asgame_state_pirate (Utilities|Casting|CastToGameStatePirate (Game|GetGameState)))
    (if (Utilities|Enum|Equal(Enum) (Variables|/Game/Blueprints/System/GameStatePirate.GameStatePirate_C|GetGameState _asgame_state_pirate) "NewEnumerator0")
      (CallFunction|SetReady))))

(fn ConstructionScript)