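; PlayerStatePirate is the player state that gives each player a color slot from the shared ColorDefinitions array on GameStatePirate.
; On BeginPlay it finds the first unused definition, marks it used and stores the index in ColorDefinitionId.
; On Destroyed it marks that slot unused again so it can be reclaimed.
; It also declares a NumberOfChests variable, which these graphs leave untouched.
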(event EventBeginPlay
  (bind _array_index (CallFunction|GetFirstUnsedDefinitionColor))
  (Utilities|Struct|SetmembersinColorDefinition (Utilities|Array|Get(acopy) (Variables|/Game/Blueprints/System/GameStatePirate.GameStatePirate_C|GetColorDefinitions (.AsGame%20State%20Pirate (Utilities|Casting|CastToGameStatePirate (Game|GetGameState)))) _array_index) true)
  (Variables|Default|SetColorDefinitionId _array_index))

(event EventTick
  (params (DeltaSeconds :type Float%20%28single-precision%29)))

(event EventDestroyed
  (Utilities|Struct|SetmembersinColorDefinition (Utilities|Array|Get(acopy) (Variables|/Game/Blueprints/System/GameStatePirate.GameStatePirate_C|GetColorDefinitions (.AsGame%20State%20Pirate (Utilities|Casting|CastToGameStatePirate (Game|GetGameState)))) (Variables|Default|GetColorDefinitionId)) false))

(fn ConstructionScript)

(fn GetFirstUnsedDefinitionColor
  (bind (_array_element _array_index) (Utilities|Array|ForEachLoopwithBreak (Variables|/Game/Blueprints/System/GameStatePirate.GameStatePirate_C|GetColorDefinitions (.AsGame%20State%20Pirate (Utilities|Casting|CastToGameStatePirate (Game|GetGameState)))))
    (:LoopBody
      (if (not (.Used (Utilities|Struct|BreakColorDefinition _array_element)))
        (return _array_index)))))