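; Server-side spawner that places and removes the deposit zone in response to pirate game mode spawn and destroy events, storing it in GameStatePirate.
; ComputeRandomPoint line-traces between random high and low points within map limits, seeking a Landscape hit at or above zero height.
; ComputeFarPoint retries those points to keep the zone a minimum distance from player pawns, ending its check at the first invalid pawn.
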(event Custom|OnZoneSpawn
  (Networking|SwitchHasAuthority
    (:Authority
      (Development|PrintString "Hello")
      (bind _location (CallFunction|ComputeFarPoint))
      (bind _returnvalue (Game|SpawnActorfromClass "/Game/Blueprints/System/DepositZone.DepositZone_C" (Math|Transform|MakeTransform _location) "Undefined" 0 0))
      (Variables|/Game/Blueprints/System/GameStatePirate.GameStatePirate_C|SetDepositZone (.AsGame%20State%20Pirate (Utilities|Casting|CastToGameStatePirate (Game|GetGameState))) _returnvalue))))

(event Custom|OnZoneDestroy
  (bind _returnvalue (Game|GetGameState))
  (bind _asgame_state_pirate (Utilities|Casting|CastToGameStatePirate _returnvalue))
  (Networking|SwitchHasAuthority
    (:Authority
      (Actor|DestroyActor (Variables|/Game/Blueprints/System/GameStatePirate.GameStatePirate_C|GetDepositZone _asgame_state_pirate))
      (Variables|/Game/Blueprints/System/GameStatePirate.GameStatePirate_C|SetDepositZone _asgame_state_pirate 0))))

(event EventBeginPlay
  (bind _aspirate_game_mode (CallFunction|GetPirateGameMode))
  (Networking|SwitchHasAuthority
    (:Authority
      (Utilities|FlowControl|Sequence
        (:then_0
          (EventDispatchers|BindEventtoDespositZoneSpawnEvent _aspirate_game_mode (delegate Custom|OnZoneSpawn)))
        (:then_1
          (EventDispatchers|BindEventtoDespositZoneDestroyEvent _aspirate_game_mode (delegate Custom|OnZoneDestroy)))))))

(event Collision|EventActorBeginOverlap
  (params (OtherActor :type Actor%20Object%20Reference)))

(fn ConstructionScript)

(fn ComputeRandomPoint
  (bind _map_min_limit_x (Variables|Default|GetMap%20Min%20Limit%20X))
  (bind _map_max_limit_x (Variables|Default|GetMap%20Max%20Limit%20X))
  (bind _map_min_limit_y (Variables|Default|GetMap%20Min%20Limit%20Y))
  (bind _map_max_limit_y (Variables|Default|GetMap%20Max%20Limit%20Y))
  (bind _returnvalue (Math|Random|RandomFloatinRange _map_min_limit_y _map_max_limit_y))
  (bind _returnvalue_2 (Math|Random|RandomFloatinRange _map_min_limit_x _map_max_limit_x))
  (while true
    ;[1 1 1] Generate random transform
    (bind (_outhit _returnvalue_3) (Collision|LineTraceForObjects (Math|Vector|MakeVector _returnvalue_2 _returnvalue 1e+03) (Math|Vector|MakeVector _returnvalue_2 _returnvalue -1e+03) (Utilities|Array|MakeArray "ObjectTypeQuery1") false 0 "None"))
    (if _returnvalue_3
      (Utilities|Casting|CastToLandscape (.HitActor (Collision|BreakHitResult _outhit)))
      (if (>= (.Z (Math|Vector|BreakVector (.ImpactPoint (Collision|BreakHitResult _outhit)))) 0.0)
        (return (Math|Transform|MakeTransform (.ImpactPoint (Collision|BreakHitResult _outhit))))))))

(fn ComputeFarPoint
  (LocalVariables|SetAllPlayerGood false)
  (while (not (LocalVariables|GetAllPlayerGood))
    (LocalVariables|SetAllPlayerGood true)
    (bind _randtransform (CallFunction|ComputeRandomPoint))
    (LocalVariables|SetResTransform _randtransform)
    (bind _array_element (Utilities|Array|ForEachLoopwithBreak (Variables|/Script/Engine.GameStateBase|GetPlayerArray (Game|GetGameState)) :!label _label)
      (:LoopBody
        (Utilities|IsValid (Variables|/Script/Engine.PlayerState|GetPawnPrivate _array_element)
          (:Is%20Valid
            (Development|PrintString (Utilities|String|ToString(Float) (Math|Vector|Distance(Vector) (.Location (Math|Transform|BreakTransform _randtransform)) (Transformation|GetActorLocation (Variables|/Script/Engine.PlayerState|GetPawnPrivate _array_element)))) true true "(R=1.000000,G=0.000000,B=0.061523,A=1.000000)")
            (if (< (Math|Vector|Distance(Vector) (.Location (Math|Transform|BreakTransform _randtransform)) (Transformation|GetActorLocation (Variables|/Script/Engine.PlayerState|GetPawnPrivate _array_element))) (Variables|Default|GetMinDistanceFromPlayers))
              (LocalVariables|SetAllPlayerGood false)
              (goto _label Break)))
          (:Is%20Not%20Valid
            (goto _label Break))))))
  (return (.Location (Math|Transform|BreakTransform (LocalVariables|GetResTransform)))))