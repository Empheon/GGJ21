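; PirateCharacter is the player pawn that walks on world axes, uses interactibles, and carries, throws and banks treasure chests.
; Stacked chests chain-attach upward from StackPoint through each chest's socket, tracked in the ChestStack array.
; Dig and Shoot input route through server-named events; shooting detaches and throws the top chest, and chest hits knock the pirate back.
; Entering a deposit zone adds the stack count to PlayerStatePirate and destroys the carried chests.
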(event Custom|OnChestStacked
  (params (Chest :type Chest%20Object%20Reference))
  (bind _cheststack (Variables|Default|GetChestStack))
  (bind _returnvalue (Utilities|Array|Length _cheststack))
  ;[1 1 1] Stack
  (Default|OnChestStacked Chest)
  (if (== _returnvalue 0)
    (Transformation|AttachComponentToComponent Chest (Variables|Components|GetStackPoint) "None" "SnapToTarget" "SnapToTarget" "SnapToTarget" true)
    (else
      (Transformation|AttachActorToActor Chest (Utilities|Array|Get(acopy) (Variables|Default|GetChestStack) (- _returnvalue 1)) "StackPoint" "SnapToTarget" "SnapToTarget" "SnapToTarget" true)))
  (Utilities|Array|Add (Variables|Default|GetChestStack) Chest))

(event Custom|InteractServer
  (bind _currentinteractible (Variables|Default|GetCurrentInteractible))
  (Utilities|IsValid _currentinteractible
    (:Is%20Valid
      (Class|IInteractible|OnUse(Message) _currentinteractible self))))

(event Custom|ShootServer
  ;[1 1 1] Shoot
  (if (> (Utilities|Array|Length (Variables|Default|GetChestStack)) 0)
    (CallFunction|ShootAll)))

(event Custom|ShootAll
  (bind _cheststack (Variables|Default|GetChestStack))
  (bind _chestthrowspawnpoint (Variables|Default|GetChestThrowSpawnPoint))
  (bind _returnvalue (Utilities|Array|Length _cheststack))
  (bind _returnvalue_2 (- _returnvalue 1))
  (bind _output (Utilities|Array|Get(acopy) _cheststack _returnvalue_2))
  ;[1 1 1] Shoot
  (if (== _returnvalue 1)
    (Transformation|DetachFromComponent (Variables|/Script/Engine.Actor|GetRootComponent _output) "KeepRelative" "KeepRelative" "KeepRelative" true)
    (else
      (Transformation|DetachFromActor _output "KeepRelative" "KeepRelative" "KeepRelative")))
  (Utilities|FlowControl|Sequence
    (:then_0
      ;[1 1 1] Throw Chest
      (Transformation|SetActorLocationAndRotation _output (Transformation|GetWorldLocation _chestthrowspawnpoint) (Transformation|GetWorldRotation _chestthrowspawnpoint) false true)
      (Default|OnThrow _output (Math|Vector|GetForwardVector _chestthrowspawnpoint) self))
    (:then_1
      (Utilities|Array|RemoveIndex (Variables|Default|GetChestStack) _returnvalue_2))))

(event Custom|OnHitChest
  (params (Dir :type Vector))
  (bind _charactermovement (Variables|Character|GetCharacterMovement))
  (Physics|AddImpulse _charactermovement (* Dir (Variables|Default|GetImpactImpulse)) true)
  (Physics|AddImpulse _charactermovement "0,0.000000,200.000000" true))

(event Custom|OnEnterDepositZone
  (bind _cheststack (Variables|Default|GetChestStack))
  ;[1 1 1] Deposit chests in zone
  (bind _asplayer_state_pirate (Utilities|Casting|CastToPlayerStatePirate (Variables|GetPlayerState)))
  (Variables|/Game/Blueprints/System/PlayerStatePirate.PlayerStatePirate_C|SetNumberOfChests _asplayer_state_pirate (+ (Variables|/Game/Blueprints/System/PlayerStatePirate.PlayerStatePirate_C|GetNumberOfChests _asplayer_state_pirate) (Utilities|Array|Length (Variables|Default|GetChestStack))))
  (bind _arrayelement (Utilities|Array|ReverseforEachLoop _cheststack)
    (:LoopBody
      (Actor|DestroyActor _arrayelement))
    (:Completed
      (Utilities|Array|Clear _cheststack))))

(event Input|ActionEvents|InputActionDig
  (params (Key :type Key%20Structure :default "None"))
  (:Pressed
    (Utilities|IsValid (Variables|Default|GetCurrentInteractible)
      (:Is%20Valid
        (CallFunction|InteractServer)))))

(event Input|ActionEvents|InputActionShoot
  (params (Key :type Key%20Structure :default "None"))
  ;[1 1 1] Shoot
  (:Pressed
    (if (> (Utilities|Array|Length (Variables|Default|GetChestStack)) 0)
      (CallFunction|ShootServer))))

(event Input|AxisEvents|InputAxisMoveForward
  (params (AxisValue :type Float%20%28single-precision%29))
  (Pawn|Input|AddMovementInput "1.000000,0.000000,0.000000" AxisValue false))

(event Input|AxisEvents|InputAxisMoveRight
  (params (AxisValue :type Float%20%28single-precision%29))
  (Pawn|Input|AddMovementInput "0.000000,1.000000,0.000000" AxisValue false))

(fn ConstructionScript)